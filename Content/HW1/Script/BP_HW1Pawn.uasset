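; BP_HW1Pawn is a pawn that controls a test rigid body through key presses.
; On BeginPlay it finds the first actor tagged HW1Actor and caches its CustomRigidbodyComponent, printing an error if no tagged actor exists.
; R resets that body to a fixed position and rotation with simulation off, while L enables simulation and launches it with a preset velocity.
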(event EventBeginPlay
  (bind _outactors (Actor|GetAllActorswithTag "HW1Actor"))
  (if (Utilities|Array|IsValidIndex _outactors)
    (if (Utilities|Array|IsValidIndex (Actor|GetComponentsByClass (Utilities|Array|Get(acopy) _outactors) "/Script/Games103.CustomRigidbodyComponent"))
      (Variables|Default|SetCustomRigidbody (Utilities|Array|Get(acopy) (Actor|GetComponentsByClass (Utilities|Array|Get(acopy) _outactors) "/Script/Games103.CustomRigidbodyComponent"))))
    (else
      (Development|PrintString "Can not find actors with CustomRigidbodyComponent" true true "(R=1.000000,G=0.000000,B=0.000000,A=1.000000)"))))

(event Input|KeyboardEvents|R
  (params (Key :type Key%20Structure :default "None"))
  (bind _customrigidbody (Variables|Default|GetCustomRigidbody))
  (:Pressed
    (Utilities|IsValid _customrigidbody
      (:Is%20Valid
        (Class|CustomRigidbodyComponent|Reset _customrigidbody (Math|Vector|MakeVector 8e+01 -2.3e+02 1.9e+02) (Class|KismetMathLibrary|QuatMakefromEuler (Math|Vector|MakeVector -1e+02 0.0 0.0)))
        (Variables|/Script/Games103.CustomRigidbodyComponent|SetbEnableSimulation _customrigidbody false)))))

(event Input|KeyboardEvents|L
  (params (Key :type Key%20Structure :default "None"))
  (bind _customrigidbody (Variables|Default|GetCustomRigidbody))
  (:Pressed
    (Utilities|IsValid _customrigidbody
      (:Is%20Valid
        (Variables|/Script/Games103.CustomRigidbodyComponent|SetbEnableSimulation _customrigidbody true)
        (Class|CustomRigidbodyComponent|ApplyVelocity _customrigidbody (Math|Vector|MakeVector 0.0 -1e+03 3e+02))))))

(fn ConstructionScript)